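; Falling platform Blueprint that drops some time after something hits it.
; A Hit sets FallDown, which lets Tick count Wait down by delta time while printing debug values.
; When Wait runs out, MoveComponentTo lowers Platfrm 500 units using world location as the relative target, followed by a second move with no component connected.
; Wait and FallDown then reset for the next hit.
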(event `self.ReceiveTick`
  (params (DeltaSeconds :type "Float (single-precision)"))
  (bind _platfrm (`self.Platfrm`))
  (bind _x (.x (`SceneComponent.K2_GetComponentLocation` _platfrm)))
  (bind _y (.y (`SceneComponent.K2_GetComponentLocation` _platfrm)))
  (bind _z (.z (`SceneComponent.K2_GetComponentLocation` _platfrm)))
  (if (`self.FallDown`)
    (bind _output_get (set `self.Wait` (- (`self.Wait`) DeltaSeconds)))
    (`KismetSystemLibrary.PrintString` (`KismetStringLibrary.Conv_DoubleToString` _output_get))
    (bind _output_get_2 (set `self.FallDown` (>= _output_get 0.0)))
    (`KismetSystemLibrary.PrintString` (`KismetStringLibrary.Conv_BoolToString` _output_get_2))
    (if (not (`self.FallDown`))
      (`KismetSystemLibrary.MoveComponentTo` _platfrm (`KismetMathLibrary.MakeVector` _x _y (- _z 500.0)) (struct) false false 2.0)
      (`KismetSystemLibrary.MoveComponentTo` null (`KismetMathLibrary.MakeVector` _x _y _z) (struct) false false 2.0)
      (set `self.Wait` 10.0)
      (set `self.FallDown` false))))

(event `self.ReceiveHit`
  (params (MyComp :type "PrimitiveComponent Object Reference") (Other :type "Actor Object Reference") (OtherComp :type "PrimitiveComponent Object Reference") (bSelfMoved :type Boolean) (HitLocation :type "Vector Structure") (HitNormal :type "Vector Structure") (NormalImpulse :type "Vector Structure") (Hit :type "HitResult Structure (by ref)"))
  (`KismetSystemLibrary.PrintString` (`KismetSystemLibrary.GetDisplayName` Other))
  (set `self.FallDown` true))

(fn `UserConstructionScript`)